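; Interactable fridge actor in the grab system that toggles its door open and closed on each Use event.
; A looping MultiGate alternates between playing and reversing a Timeline that lerps the door's yaw, starting the matching open or close audio.
; A DoOnce blocks repeated use until a short Delay, triggered from the Timeline update, resets it.
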(event EventUse
  (Utilities|FlowControl|DoOnce false :!label _label
    (:Completed
      (Utilities|FlowControl|MultiGate false true -1
        (:Out%200
          (Audio|Components|Audio|Play (Variables|Default|GetOpenFridge) 0.0)
          (bind _openclose (Timeline|Timeline Play)
            (:Update
              (Transformation|SetRelativeRotation (Variables|Default|GetFridgeDoor) (Math|Rotator|MakeRotator 0.0 0.0 (Math|Float|Lerp 0.0 -1.1e+02 _openclose)) false false)
              (Utilities|FlowControl|Delay 0.6)
              (goto _label Reset))))
        (:Out%201
          (Audio|Components|Audio|Play (Variables|Default|GetCloseFridge) 0.0)
          (Timeline|Timeline Reverse))))))

(fn ConstructionScript)