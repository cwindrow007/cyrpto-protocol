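; Usable window actor that slides open by itself after being shut.
; While Shut is set, Tick starts a random 5 to 15 second Delay, then clears the flag and plays the WindowUp timeline to raise the window along relative Z.
; Use on an open window sets Shut and reverses the same timeline to lower it, restarting the cycle.
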(event EventUse
  (if (not (Variables|Default|GetShut?))
    (Variables|Default|SetShut? true)
    (Utilities|FlowControl|Sequence
      (:then_0
        (bind _windowup_down (Timeline|WindowUp Reverse)
          (:Update
            (Transformation|SetRelativeLocation (Variables|Default|GetWindow) (Math|Vector|MakeVector 0.0 0.0 (Math|Float|Lerp 0.0 75.0 _windowup_down)) false false)))))))

(event EventTick
  (params (DeltaSeconds :type Float%20%28single-precision%29))
  (if (Variables|Default|GetShut?)
    (Utilities|FlowControl|Delay (Math|Random|RandomFloatinRange 5.0 15.0))
    (Variables|Default|SetShut? false)
    (bind _windowup_down (Timeline|WindowUp Play)
      (:Update
        (Transformation|SetRelativeLocation (Variables|Default|GetWindow) (Math|Vector|MakeVector 0.0 0.0 (Math|Float|Lerp 0.0 75.0 _windowup_down)) false false)))))

(fn ConstructionScript)