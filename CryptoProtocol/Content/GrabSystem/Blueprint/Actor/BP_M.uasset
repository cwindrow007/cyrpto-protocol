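; Interactable actor that toggles the player's view between their character and a monitor camera actor (BPmonitorcamera).
; Any actor overlap enables player input on it, and ending overlap disables it.
; While overlapping, Use drives a looping MultiGate that alternately blends to the camera with look input ignored, or back to the character with look restored.
; A DoOnce, reset after a delay matching the blend, blocks retriggering mid-transition.
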(event EventUse
  (bind _returnvalue (Game|GetPlayerCharacter 0))
  (bind _returnvalue_2 (Game|GetPlayerController 0))
  (if (Variables|Default|GetOVERLAPPING)
    (Utilities|FlowControl|DoOnce false :!label _label
      (:Completed
        (Utilities|FlowControl|MultiGate false true -1
          (:Out%200
            (Development|PrintString "1")
            (bind _asbp_third_person_character (Utilities|Casting|CastToBP_ThirdPersonCharacter _returnvalue))
            (if (Utilities|IsValid _asbp_third_person_character)
              (bind _asplayer_controller (Utilities|Casting|CastToPlayerController (Pawn|GetController _asbp_third_person_character)))
              (if (Utilities|IsValid _asplayer_controller)
                (bind _returnvalue_3 (Actor|GetActorOfClass "/Game/GrabSystem/Blueprint/Actor/BPmonitorcamera.BPmonitorcamera_C"))
                (Game|Player|SetViewTargetwithBlend _asplayer_controller _returnvalue_3 0.6 "VTBlend_Linear" 0.0 false)
                (Input|SetIgnoreLookInput _returnvalue_2 true)
                (Utilities|FlowControl|Delay 0.6)
                (goto _label Reset))))
          (:Out%201
            (Development|PrintString "2")
            (bind _asbp_third_person_character_2 (Utilities|Casting|CastToBP_ThirdPersonCharacter _returnvalue))
            (if (Utilities|IsValid _asbp_third_person_character_2)
              (bind _asplayer_controller_2 (Utilities|Casting|CastToPlayerController (Pawn|GetController _asbp_third_person_character_2)))
              (if (Utilities|IsValid _asplayer_controller_2)
                (Game|Player|SetViewTargetwithBlend _asplayer_controller_2 _asbp_third_person_character_2 0.6 "VTBlend_Linear" 0.0 false)
                (Input|ResetIgnoreLookInput _returnvalue_2)
                (Utilities|FlowControl|Delay 0.6)
                (goto _label Reset)))))))))

(event Collision|EventActorBeginOverlap
  (params (OtherActor :type Actor%20Object%20Reference))
  (Variables|Default|SetOVERLAPPING true)
  (Input|EnableInput (Game|GetPlayerController 0)))

(event Collision|EventActorEndOverlap
  (params (OtherActor :type Actor%20Object%20Reference))
  (Variables|Default|SetOVERLAPPING false)
  (Input|DisableInput (Game|GetPlayerController 0)))

(fn ConstructionScript)