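; Interactive router actor that toggles the player between normal play and a RouterCam close-up each time it is used.
; Use drives a looping MultiGate that freezes or restores movement and look input while blending the view target.
; A DoOnce, reset after each blend, blocks re-triggering mid-transition.
; Tick runs a random long Delay, then applies the Color variable to the Wi-Fi light through a new dynamic material.
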(event EventUse
  (bind _returnvalue (Game|GetPlayerCharacter 0))
  (bind _returnvalue_2 (Game|GetPlayerCharacter 0))
  (bind _returnvalue_3 (Game|GetPlayerController 0))
  (bind _charactermovement (Variables|/Script/Engine.Character|GetCharacterMovement _returnvalue))
  (Utilities|FlowControl|DoOnce false :!label _label
    (:Completed
      (Utilities|FlowControl|MultiGate false true -1
        (:Out%200
          (Pawn|Components|CharacterMovement|SetMovementMode _charactermovement "MOVE_None" 0)
          (bind _asbp_third_person_character (Utilities|Casting|CastToBP_ThirdPersonCharacter _returnvalue_2))
          (if (Utilities|IsValid _asbp_third_person_character)
            (bind _asplayer_controller (Utilities|Casting|CastToPlayerController (Pawn|GetController _asbp_third_person_character)))
            (if (Utilities|IsValid _asplayer_controller)
              (bind _returnvalue_4 (Actor|GetActorOfClass "/Game/GrabSystem/Blueprint/Actor/RouterCam.RouterCam_C"))
              (Game|Player|SetViewTargetwithBlend _asplayer_controller _returnvalue_4 0.6 "VTBlend_Linear" 0.0 false)
              (Input|SetIgnoreLookInput _returnvalue_3 true)
              (Utilities|FlowControl|Delay 0.6)
              (goto _label Reset))))
        (:Out%201
          (Pawn|Components|CharacterMovement|SetMovementMode _charactermovement "MOVE_Walking" 0)
          (bind _asbp_third_person_character_2 (Utilities|Casting|CastToBP_ThirdPersonCharacter _returnvalue_2))
          (if (Utilities|IsValid _asbp_third_person_character_2)
            (bind _asplayer_controller_2 (Utilities|Casting|CastToPlayerController (Pawn|GetController _asbp_third_person_character_2)))
            (if (Utilities|IsValid _asplayer_controller_2)
              (Game|Player|SetViewTargetwithBlend _asplayer_controller_2 _asbp_third_person_character_2 0.6 "VTBlend_Linear" 0.0 false)
              (Input|ResetIgnoreLookInput _returnvalue_3)
              (Utilities|FlowControl|Delay 0.6)
              (goto _label Reset))))))))

(event EventTick
  (params (DeltaSeconds :type Float%20%28single-precision%29))
  (Utilities|FlowControl|Delay (Math|Random|RandomFloatinRange 5e+01 5e+02))
  (bind _returnvalue (Rendering|Material|CreateDynamicMaterialInstance (Variables|Default|GetGreenLightsWIFI) 0 "/Game/Materials/green.green" "None" :!class /Script/Engine.PrimitiveComponent))
  (Rendering|Material|SetVectorParameterValue _returnvalue "color" (Variables|Default|Getcolor) :!class /Script/Engine.MaterialInstanceDynamic))

(fn ConstructionScript)