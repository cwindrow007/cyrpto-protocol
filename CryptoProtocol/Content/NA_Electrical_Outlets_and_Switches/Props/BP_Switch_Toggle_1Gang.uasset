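; One-gang toggle light switch prop that switches linked lights on and off when used.
; Use alternates through a looping MultiGate; each branch plays the flip sound, toggles visibility on four referenced light holders' components and sets the toggle's pitch.
; Visibility is flipped rather than set, so on/off follows each light's starting state.
; Dynamic-material code for faceplate, screw and switch finishes is unconnected, and the construction script is empty.
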(event EventBeginPlay)

(event Collision|EventActorBeginOverlap
  (params (OtherActor :type Actor%20Object%20Reference)))

(event EventTick
  (params (DeltaSeconds :type Float%20%28single-precision%29)))

(event EventUse
  (bind _lightholder (Variables|Default|GetLightHolder))
  (bind _bp_switch_toggle (Variables|Default|GetBP_Switch_Toggle))
  (bind _lightswitchflip (Variables|Default|GetLightSwitchFlip))
  (bind _rectlightcomponent (Variables|/Script/Engine.RectLight|GetRectLightComponent _lightholder))
  (Utilities|FlowControl|MultiGate false true -1
    (:Out%200
      (Audio|Components|Audio|Play _lightswitchflip 0.0)
      (Rendering|ToggleVisibility _rectlightcomponent false)
      (Transformation|SetRelativeRotation _bp_switch_toggle (Math|Rotator|MakeRotator 0.0 -5.0 0.0) false false))
    (:Out%201
      (Audio|Components|Audio|Play _lightswitchflip 0.0)
      (Rendering|ToggleVisibility _rectlightcomponent false)
      (Transformation|SetRelativeRotation _bp_switch_toggle (Math|Rotator|MakeRotator 0.0 55.0 0.0) false false))))

(fn ConstructionScript)