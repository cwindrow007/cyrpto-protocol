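; Physics-driven six-sided die actor that rolls itself and reports the face it lands on.
; Roll teleports it to its start location with random rotation, applies a random radial impulse, then polls velocity on a looping timer.
; Once it settles, physics stops and the upward-pointing child arrow component gives the value through a map.
; A valid value fires OnRollComplete, while a crooked landing rerolls after a short delay.
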(event Custom|Start%20Roll%20Check
  (bind _returnvalue (Utilities|Time|SetTimerbyEvent (delegate Custom|Check%20If%20Stopped) 0.25 true true))
  (Variables|Default|SetRoll%20Check%20Timer _returnvalue))

(event Custom|Check%20If%20Stopped
  (if (CallFunction|HasDieStoppedMoving?)
    (Variables|Default|SetLast%20Location (CallFunction|GetLocation))
    (bind _output_get (Variables|Default|SetIs%20Rolling? false))
    (Physics|SetSimulatePhysics (Variables|Default|GetDie) _output_get)
    (Utilities|Time|ClearandInvalidateTimerbyHandle (Variables|Default|GetRoll%20Check%20Timer))
    (bind _final_value (CallFunction|GetDieValue))
    (if (< _final_value 1) ; Maybe this die landed crooked? If so, redo.
      (Utilities|FlowControl|Delay 1.0)
      (CallFunction|Roll)
      (else
        (Default|CallOnRollComplete _final_value)))))

(event EventBeginPlay
  (Variables|Default|SetInitial%20Location (Transformation|GetActorLocation))
  (CallFunction|PopulateArrowValues))

(event EventShow
  (Rendering|SetVisibility (Variables|Default|GetDie) true false))

(event EventHide
  (Rendering|SetVisibility (Variables|Default|GetDie) false false))

(event EventRoll
  (Class|BPIDiceFunctionality|Show(Message) self)
  (Variables|Default|SetIs%20Rolling? true)
  (Physics|SetSimulatePhysics (Variables|Default|GetDie) true)
  (bind _output_get (Variables|Default|SetLast%20Location (Variables|Default|GetInitial%20Location)))
  (Transformation|SetActorLocationAndRotation _output_get (Math|Random|RandomRotator true) false true)
  (Physics|AddRadialImpulse (Variables|Default|GetDie) (Variables|Default|GetLast%20Location) 5e+01 (CallFunction|GetRandomRadialImpulseStrength) "RIF_Constant" false)
  (CallFunction|StartRollCheck))

(fn ConstructionScript)

(fn GetRandomRadialImpulseStrength
  (return (Math|Random|RandomFloatinRange (Variables|Default|GetDie%20Impulse%20Min) (Variables|Default|GetDie%20Impulse%20Max))))

(fn GetLocation
  (return (Transformation|GetActorLocation)))

(fn HasDieStoppedMoving?
  (return (Utilities|Operators|EqualEqual :A (Transformation|GetVelocity) :ErrorTolerance (Variables|Default|GetDie%20Velocity%20Min))))

(fn PopulateArrowValues
  (bind _arrow_values (Variables|Default|GetArrow%20Values))
  (Utilities|Map|Clear _arrow_values) ; Must come first
  (Utilities|Map|Add _arrow_values (Variables|Default|GetArrow%201) 1)
  (Utilities|Map|Add _arrow_values (Variables|Default|GetArrow%202) 2)
  (Utilities|Map|Add _arrow_values (Variables|Default|GetArrow%203) 3)
  (Utilities|Map|Add _arrow_values (Variables|Default|GetArrow%204) 4)
  (Utilities|Map|Add _arrow_values (Variables|Default|GetArrow%205) 5)
  (Utilities|Map|Add _arrow_values (Variables|Default|GetArrow%206) 6))

(fn IsArrowFacingUp?
  (params (Arrow :type Scene%20Component%20Object%20Reference))
  (return (Utilities|Operators|EqualEqual (Math|Vector|GetForwardVector Arrow) "0.000000,0.000000,1.000000" (Variables|Default|GetUpward%20Detection%20Threshold))))

(fn GetDieValue
  (for _array_element (Components|GetChildrenComponents (Variables|Default|GetDie) false)
    (if (and (CallFunction|IsArrowFacingUp? _array_element) (.bSuccess (Utilities|Casting|CastToArrowComponent _array_element)))
      (return (.Value (Utilities|Map|Find (Variables|Default|GetArrow%20Values) (.AsArrow%20Component (Utilities|Casting|CastToArrowComponent _array_element)))))))
  (return 0) ; None of the arrows are facing up; something went wrong.
)