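; Game mode for a dice game that rolls every BP_Die in the level and reports their combined total.
; On BeginPlay it gathers the dice, binds one handler to each die's roll-complete event, and shows the debug console widget.
; RollAllDice messages each stored die to roll.
; Results accumulate until every die has reported, then AllDiceRollsComplete prints the total and resets the counters.
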(event EventRollAllDice
  (Class|BPIDiceFunctionality|Hide(Message) self)
  (for _array_element (Variables|Settings|GetDice)
    (Class|BPIDiceFunctionality|Roll(Message) _array_element)))

(event EventOnSingleDieFinished
  (params (Value :type Integer))
  (CallFunction|AddtoTotalandCheckifDone Value))

(event EventBeginPlay
  (CallFunction|DetectandStoreDice (delegate EventOnSingleDieFinished))
  (CallFunction|DisplayUI))

(event EventAllDiceRollsComplete
  (params (Total%20Value :type Integer))
  (Development|PrintString (Utilities|String|Append "ROLLED: " (Utilities|String|ToString(Integer) Total%20Value)) true false "(R=1.000000,G=0.250000,B=0.000000,A=1.000000)" 5.0)
  (bind _output_get (Variables|DiceFunctionality|SetTotal%20Roll%20Value 0))
  (Variables|DiceFunctionality|SetNumber%20of%20Finished%20Dice _output_get))

(fn ConstructionScript)

(fn DisplayUI
  (bind _returnvalue (UserInterface|CreateWidget "/Game/_Dice_/UI/WBP_DebugConsole.WBP_DebugConsole_C"))
  (UserInterface|Viewport|AddtoViewport _returnvalue 0))

(fn DetectandStoreDice
  (params (OnRollComplete%20Delegate :type %20Object%20Reference%20%28by%20ref%29))
  (bind _outactors (Actor|GetAllActorsOfClass "/Game/_Dice_/Blueprints/Objects/BP_Die.BP_Die_C")) ; Get all BP_Die instances in our level
  (for _array_element _outactors
    (Utilities|Array|Add (Variables|Settings|GetDice) _array_element) ; Store each Die for reference
    (EventDispatchers|BindEventtoOnRollComplete _array_element OnRollComplete%20Delegate) ; Connect our delegate to OnRollComplete
  ))

(fn AddtoTotalandCheckifDone
  (params (Value%20Rolled :type Integer))
  (Variables|DiceFunctionality|SetTotal%20Roll%20Value (+ Value%20Rolled (Variables|DiceFunctionality|GetTotal%20Roll%20Value)))
  (bind _result (Math|Integer|IncrementInt (Variables|DiceFunctionality|GetNumber%20of%20Finished%20Dice))
    (:%20%20
      (if (== _result (Utilities|Array|Length (Variables|Settings|GetDice)))
        (CallFunction|AllDiceRollsComplete (Variables|DiceFunctionality|GetTotal%20Roll%20Value))))))